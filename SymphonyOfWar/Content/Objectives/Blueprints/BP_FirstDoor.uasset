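; BP_FirstDoor is a one-shot objective trigger that completes the player's current objective and assigns the next one.
; On BeginPlay it clears the ObjectiveComplete flag on the BP_SOWPlayerCharacter.
; When that character overlaps its Box, it sets the flag, plays a ding and removes the Box.
; After a short delay it sets the objective text to collecting Zephyr parts for the HQ portal, resets the flag and destroys itself.
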(event OnComponentBeginOverlap(Box)
  (params (OverlappedComponent :type Primitive%20Component%20Object%20Reference) (OtherActor :type Actor%20Object%20Reference) (OtherComp :type Primitive%20Component%20Object%20Reference) (OtherBodyIndex :type Integer) (bFromSweep :type Boolean) (SweepResult :type Hit%20Result%20Structure%20%28by%20ref%29))
  (bind _asbp_sowplayer_character (Utilities|Casting|CastToBP_SOWPlayerCharacter OtherActor))
  (Variables|/Game/Blueprints/BP_SOWPlayerCharacter.BP_SOWPlayerCharacter_C|SetObjectiveComplete _asbp_sowplayer_character true)
  (Audio|PlaySound2D "/Game/Objectives/Audio/320905__suzenako__the-ding.320905__suzenako__the-ding" 1.0 1.0 0.0 0 0)
  (Components|DestroyComponent (Variables|Default|GetBox))
  (Utilities|FlowControl|Delay 2.0)
  (Variables|/Game/Blueprints/BP_SOWPlayerCharacter.BP_SOWPlayerCharacter_C|SetObjective _asbp_sowplayer_character "Collect all the Zephyr parts to open the portal to HQ. Watch out for enemies!")
  (Variables|/Game/Blueprints/BP_SOWPlayerCharacter.BP_SOWPlayerCharacter_C|SetObjectiveComplete _asbp_sowplayer_character false)
  (Actor|DestroyActor))

(event EventBeginPlay
  (bind _asbp_sowplayer_character (Utilities|Casting|CastToBP_SOWPlayerCharacter (Game|GetPlayerCharacter 0)))
  (Variables|/Game/Blueprints/BP_SOWPlayerCharacter.BP_SOWPlayerCharacter_C|SetObjectiveComplete _asbp_sowplayer_character false))

(event Collision|EventActorBeginOverlap
  (params (OtherActor :type Actor%20Object%20Reference)))

(event EventTick
  (params (DeltaSeconds :type Float%20%28single-precision%29)))

(fn ConstructionScript)