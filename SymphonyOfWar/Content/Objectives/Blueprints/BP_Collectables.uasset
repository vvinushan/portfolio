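; BP_Collectables is a pickup actor that counts toward a five-item collection objective.
; When the player character overlaps its collision box, it increments that character's GotCollectables count and destroys itself.
; On the fifth pickup, it flags the player's objective complete, enables TimeEnabled and plays a ding sound.
; For other counts, it adds a W_CollectableCount widget to the viewport.
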(event OnComponentBeginOverlap(CollisionBox)
  (params (OverlappedComponent :type Primitive%20Component%20Object%20Reference) (OtherActor :type Actor%20Object%20Reference) (OtherComp :type Primitive%20Component%20Object%20Reference) (OtherBodyIndex :type Integer) (bFromSweep :type Boolean) (SweepResult :type Hit%20Result%20Structure%20%28by%20ref%29))
  (bind _asbp_sowplayer_character (Utilities|Casting|CastToBP_SOWPlayerCharacter OtherActor))
  (Variables|/Game/Blueprints/BP_SOWPlayerCharacter.BP_SOWPlayerCharacter_C|SetGotCollectables _asbp_sowplayer_character (+ (Variables|/Game/Blueprints/BP_SOWPlayerCharacter.BP_SOWPlayerCharacter_C|GetGotCollectables _asbp_sowplayer_character) 1))
  (Actor|DestroyActor)
  (if (== (Variables|/Game/Blueprints/BP_SOWPlayerCharacter.BP_SOWPlayerCharacter_C|GetGotCollectables _asbp_sowplayer_character) 5)
    (bind _asbp_sowplayer_character_2 (Utilities|Casting|CastToBP_SOWPlayerCharacter (Game|GetPlayerCharacter 0)))
    (Variables|/Game/Blueprints/BP_SOWPlayerCharacter.BP_SOWPlayerCharacter_C|SetObjectiveComplete _asbp_sowplayer_character_2 true)
    (Variables|/Game/Blueprints/BP_SOWPlayerCharacter.BP_SOWPlayerCharacter_C|SetTimeEnabled _asbp_sowplayer_character_2 true)
    (Audio|PlaySound2D "/Game/Objectives/Audio/320905__suzenako__the-ding.320905__suzenako__the-ding" 1.0 1.0 0.0 0 0)
    (Utilities|FlowControl|Delay 2.0)
    (else
      (bind _returnvalue (UserInterface|CreateWidget "/Game/Objectives/UI/W_CollectableCount.W_CollectableCount_C"))
      (bind _output_get (Variables|Default|SetWCollectableCount _returnvalue))
      (UserInterface|Viewport|AddtoViewport _output_get 0))))

(event EventBeginPlay)

(event Collision|EventActorBeginOverlap
  (params (OtherActor :type Actor%20Object%20Reference)))

(event EventTick
  (params (DeltaSeconds :type Float%20%28single-precision%29)))

(fn ConstructionScript)