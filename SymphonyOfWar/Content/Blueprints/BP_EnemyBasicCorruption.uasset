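; Basic corruption enemy that drives an overhead health bar and damages the player.
; Tick pushes Health into the W_EnemyProgressBar widget and, while IsStillDamaging is set, uses a one-second Delay to repeatedly subtract player health and play an attack animation.
; Nothing in this graph sets that flag.
; Return-to-base movement and animation-mode reset logic are left unconnected and never run.
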(event EventBeginPlay)

(event Collision|EventActorBeginOverlap
  (params (OtherActor :type Actor%20Object%20Reference)))

(event EventTick
  (params (DeltaSeconds :type Float%20%28single-precision%29))
  (Utilities|FlowControl|Sequence
    (:then_0
      (bind _asw_enemy_progress_bar (Utilities|Casting|CastToW_EnemyProgressBar (UserInterface|GetUserWidgetObject (Variables|Default|GetEnemyHealthBar))))
      (Progress|SetPercent (Variables|/Game/HUD/UI/W_EnemyProgressBar.W_EnemyProgressBar_C|GetEnemyHealthBar _asw_enemy_progress_bar) (Variables|Default|GetHealth)))
    (:then_1
      (if (Variables|Default|GetIsStillDamaging)
        (Utilities|FlowControl|Delay 1.0)
        (bind _asbp_sowplayer_character (Utilities|Casting|CastToBP_SOWPlayerCharacter (Game|GetPlayerCharacter 0)))
        (Variables|/Script/SymphonyOfWar.SOWPlayerCharacter|SetHealth _asbp_sowplayer_character (- (Variables|/Script/SymphonyOfWar.SOWPlayerCharacter|GetHealth _asbp_sowplayer_character) 0.05))
        (Components|Animation|PlayAnimation (Variables|Default|GetEnemyMesh) "/Game/UndeadPack/SkeletonEnemy/Animations/Anim_Attack_1.Anim_Attack_1" false)))))

(fn ConstructionScript)