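; Game mode that randomizes which pre-placed collectables and final doors remain in the level at BeginPlay.
; For each type, it gathers all actors of the class, shuffles them, and destroys the surplus beyond the SpawnCollectables or SpawnDoors count.
; MaxCollectables and MaxDoors start at the found totals and decrement with each removal, ending as the surviving counts.
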(event EventBeginPlay
  (Utilities|FlowControl|Sequence
    (:then_0
      (bind _outactors (Actor|GetAllActorsOfClass "/Game/Objectives/Blueprints/BP_Collectables.BP_Collectables_C"))
      (Utilities|Array|Shuffle _outactors)
      (Variables|Default|SetMaxCollectables (Utilities|Array|Length _outactors))
      (for _index (range 0 (- (Utilities|Array|Length _outactors) (+ (Variables|Default|GetSpawnCollectables) 1)))
        (Actor|DestroyActor (Utilities|Array|Get(acopy) _outactors _index))
        (Variables|Default|SetMaxCollectables (- (Variables|Default|GetMaxCollectables) 1))))
    (:then_1
      (bind _outactors_2 (Actor|GetAllActorsOfClass "/Game/Objectives/Blueprints/BP_FinalDoor.BP_FinalDoor_C"))
      (Utilities|Array|Shuffle _outactors_2)
      (Variables|Default|SetMaxDoors (Utilities|Array|Length _outactors_2))
      (for _index_2 (range 0 (- (Utilities|Array|Length _outactors_2) (+ (Variables|Default|GetSpawnDoors) 1)))
        (Actor|DestroyActor (Utilities|Array|Get(acopy) _outactors_2 _index_2))
        (Variables|Default|SetMaxDoors (- (Variables|Default|GetMaxDoors) 1))))))

(fn ConstructionScript)